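; BP_Lich_AV is a Lich NPC Blueprint in AnimalSpawnVariety that inherits its begin-play and construction logic from its parent.
; EquipWeapons looks up a random slot item in ItemTable, flagging two-handed weapons or shield blocking from its archetype.
; The returned item comes from a separately evaluated random pick, so it can differ from the one that set the flags.
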(event EventBeginPlay
  (|CallParentFunction))

(event Collision|EventActorBeginOverlap
  (params (OtherActor :type Actor%20Object%20Reference)))

(event EventTick
  (params (DeltaSeconds :type Float%20%28single-precision%29))
  (|CallParentFunction 0.0))

(fn ConstructionScript
  (|CallParentFunction))

(fn EquipWeapons
  (params (ItemSlotArray :type Array%20of%20Integers))
  (bind _returnvalue (Utilities|Array|Length ItemSlotArray))
  (bind _returnvalue_2 (- _returnvalue 1))
  (bind _returnvalue_3 (Math|Random|RandomIntegerinRange 0 _returnvalue_2))
  (bind _item (Utilities|Array|Get(acopy) ItemSlotArray _returnvalue_3))
  (bind _returnvalue_4 (Utilities|GetDataTableRow "/Game/Items/ItemTable.ItemTable" (Utilities|String|StringToName (Utilities|String|ToString(Integer) _item)))
    (:then
      (if (Utilities|Enum|Equal(Enum) (.WeaponArcheType (Utilities|Struct|BreakItemTableRow _returnvalue_4)) "TwoHanded")
        (Variables|Default|SetHasTwoHandedWeapon true)
        (elif (Utilities|Enum|Equal(Enum) (.WeaponArcheType (Utilities|Struct|BreakItemTableRow _returnvalue_4)) "Shield")
          (Variables|Default|SetHasBlock true))))
    (:RowNotFound
      _))
  (return _item))