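; Entertainer thrall component that makes its character dance when idle and buffs nearby player pawns, driven by the server.
; A looping timer, marked as a temporary solution, starts a random dance emote after accumulated stationary time without a target, and stops it on movement.
; Tick queries the cached PlayerPawnRegistry by radius and applies the buff class loaded from ThrallInfo, falling back to entertainer health regen.
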(event Custom|UpdateBehaviour
  (bind _returnvalue (Components|GetOwner))
  (bind _returnvalue_2 (Components|GetOwner))
  (bind _returnvalue_3 (Actor|GetComponentbyClass _returnvalue_2 "/Script/ConanSandbox.EmoteController"))
  (bind _returnvalue_4 (Transformation|GetVelocity _returnvalue))
  (bind _returnvalue_5 (Math|Vector|Equal(Vector) _returnvalue_4 "0, 0, 0" 0.0001))
  ;[1 1 1] TEMP SOLUTION: Will make thralls use same system as NPCs (in trunk/dev first)
  (if (Default|InSubstate (Variables|Default|GetOwningBPChar) "NewEnumerator5")
    (if (not _returnvalue_5)
      (Utilities|IsValid _returnvalue_3
        (:Is%20Valid
          (Class|EmoteController|StopEmote _returnvalue_3 false))))
    (elif _returnvalue_5
      (bind _output_get (Variables|Default|SetTimeSinceStoppedMoving (+ (Variables|Default|GetTimeSinceStoppedMoving) 1.0)))
      (if (>= _output_get 3.0)
        (if (not (Class|TargetDistributionComponent|HasTarget (Variables|/Script/ConanSandbox.ConanCharacter|GetTargetingComponent (Variables|Default|GetOwningBPChar))))
          (CallFunction|StartMainTask)
          (Variables|Default|SetTimeSinceStoppedMoving 0.0))))))

(event EventBeginPlay
  (|CallParentFunction)
  (if (Variables|Default|GetIsABrush)
    (Components|Tick|SetComponentTickEnabled false)
    (else
      (Utilities|FlowControl|Sequence
        (:then_0
          (if (Networking|IsServer)
            (bind _outactors (Actor|GetAllActorsOfClass "/Script/ConanSandbox.ConanWorldSettings"))
            (bind _returnvalue (Class|ConanWorldSettings|GetPlayerPawnRegistry (Utilities|Array|Get(acopy) _outactors)))
            (Variables|Default|SetPlayerPawnRegistry _returnvalue)
            (else
              (Components|Tick|SetComponentTickEnabled false))))
        (:then_1
          (bind _asbase_bpchar (Utilities|Casting|CastToBaseBPChar (Components|GetOwner)))
          (Variables|Default|SetOwningBPChar _asbase_bpchar))
        (:then_2
          (if (Networking|IsServer)
            (Utilities|Time|SetTimerbyEvent (delegate Custom|UpdateBehaviour) 1.0 true)))))))

(event EventTick
  (params (DeltaSeconds :type Float%20%28single-precision%29))
  (|CallParentFunction DeltaSeconds)
  (if (not (Variables|Default|GetIsABrush))
    (if (Networking|IsServer)
      (bind _returnvalue (Class|PlayerPawnRegistry|GetPawnsWithinDistance (Variables|Default|GetPlayerPawnRegistry) (Transformation|GetActorLocation (Components|GetOwner)) 1e+03))
      (for _array_element _returnvalue
        (CallFunction|ApplyEntertainerBuff _array_element)))))

(fn StartMainTask
  (bind _returnvalue (Components|GetOwner))
  (bind _returnvalue_2 (Math|Random|RandomInteger 3))
  (bind _returnvalue_3 (Actor|GetComponentbyClass _returnvalue "/Script/ConanSandbox.EmoteController"))
  (Utilities|IsValid _returnvalue_3
    (:Is%20Valid
      (if (Networking|IsServer)
        (if (== _returnvalue_2 0)
          (Class|EmoteController|StartEmote _returnvalue_3 "DanceSexy")
          (elif (== _returnvalue_2 1)
            (Class|EmoteController|StartEmote _returnvalue_3 "DanceSexy")
            (else
              (Class|EmoteController|StartEmote _returnvalue_3 "DanceBelly"))))
        (return true)
        (else
          (return false))))))

(fn ApplyEntertainerBuff
  (params (Target :type Actor%20Object%20Reference))
  (bind _returnvalue (Actor|GetComponentsByClass Target "/Game/Systems/Buffs/00_BP_AC_BuffSystem.00_BP_AC_BuffSystem_C"))
  (bind _returnvalue_2 (Components|GetOwner))
  (bind _item (Utilities|Array|Get(acopy) _returnvalue))
  (bind _controller (CallFunction|GetControllerfromActor _returnvalue_2))
  (if (> (Utilities|Array|Length _returnvalue) 0)
    (bind _returnvalue_3 (Class|FuncomGenericLibrary|LoadClassfromPath (.thrallbuff (Variables|Default|GetThrallInfo))))
    (bind _as01_bp_ac_buff_master (Utilities|Casting|CastTo01_BP_AC_Buff_MasterClass _returnvalue_3)
      (:then
        (Default|AddBuff _item _as01_bp_ac_buff_master _returnvalue_2 1 _controller))
      (:CastFailed
        (Default|AddBuff _item "/Game/Systems/Buffs/HealthRegen/BP_AC_Buff_Entertainer_HealthRegen.BP_AC_Buff_Entertainer_HealthRegen_C" _returnvalue_2 1 _controller)))))